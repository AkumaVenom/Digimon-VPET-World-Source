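; Automatic flamethrower turret that tracks characters it sees and fires while they stay in view and ammo lasts.
; PawnSensing refreshes an in-range flag, and Tick turns the tray and barrel toward the target with RInterpTo and updates a screen widget.
; Gate and retriggerable-delay loops drive ammo drain, flame effects and box-overlap hits on characters or bots.
; Hits attach fire particles but only print "Hit", applying no damage.
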(event `self.ReceiveTick`
  (params (DeltaSeconds :type "Float (single-precision)"))
  (set `self.delta time` DeltaSeconds)
  (if (not (`self.OFF`))
    (`self.Turret rotation`)
    (`self.fire action`)
    (set `/Game/Automatic_FlameThrower_Turret/UI/Turret_Screen.ammo ` (`self.ammo`) (stale `self.ReceiveBeginPlay` _returnvalue))
    (set `/Game/Automatic_FlameThrower_Turret/UI/Turret_Screen.Max Ammo` (`self.max ammo`) (stale `self.ReceiveBeginPlay` _returnvalue))
    (set `/Game/Automatic_FlameThrower_Turret/UI/Turret_Screen.health` (`self.Health`) (stale `self.ReceiveBeginPlay` _returnvalue))))

(event `self.ReceiveBeginPlay`
  (bind _returnvalue (`|CreateWidget` "/Game/Automatic_FlameThrower_Turret/UI/Turret_Screen.Turret_Screen_C"))
  (`WidgetComponent.SetWidget` (`self.Widget`) _returnvalue)
  (set `self.Get Base Position` (`SceneComponent.K2_GetComponentRotation` (`self.DefaultSceneRoot`))))

(event `self.PawnSensing.OnSeePawn`
  (params (Pawn :type "Pawn Object Reference"))
  ;[1 1 1] check enemy area
  (bind _ascharacter (cast `Character` Pawn))
  (set `self.player` _ascharacter)
  (`|ExecutionSequence`
    (:`then_0`
      (set `self.in range` true))
    (:`then_1`
      (`KismetSystemLibrary.RetriggerableDelay` 0.15)
      (set `self.in range` false))))

(event `Turret rotation`
  (bind _get_base_position_roll (`KismetMathLibrary.BreakRotator` (`self.Get Base Position`)))
  (bind _flamethrower_turret (`self.flameThrower_turret`))
  (bind _returnvalue (`self.K2_GetActorLocation` (`self.player`)))
  (bind _returnvalue_2 (`self.K2_GetActorLocation` (`self.player`)))
  (bind (_returnvalue_roll _returnvalue_pitch _returnvalue_yaw) (`KismetMathLibrary.BreakRotator` (`SceneComponent.K2_GetComponentRotation` (`self.turret_tray`))))
  (bind (_returnvalue_roll_2 _returnvalue_pitch_2 _returnvalue_yaw_2) (`KismetMathLibrary.BreakRotator` (`KismetMathLibrary.RInterpTo` (`KismetMathLibrary.MakeRotator` 0.0 0.0 _returnvalue_yaw) (`KismetMathLibrary.MakeRotator` 0.0 0.0 (.yaw (`KismetMathLibrary.FindLookAtRotation` (`SceneComponent.K2_GetComponentLocation` (`self.turret_tray`)) _returnvalue_2))) (`self.delta time`) (`self.rotation speed`))))
  (bind (_returnvalue_roll_3 _returnvalue_pitch_3) (`KismetMathLibrary.BreakRotator` (`KismetMathLibrary.RInterpTo` (`SceneComponent.K2_GetComponentRotation` _flamethrower_turret) (`KismetMathLibrary.MakeRotator` 0.0 (* (.pitch (`KismetMathLibrary.FindLookAtRotation` (`SceneComponent.K2_GetComponentLocation` _flamethrower_turret) _returnvalue)) -1.0)) (`self.delta time`) (`self.rotation speed`))))
  (if (`self.in range`)
    (`|ExecutionSequence`
      (:`then_0`
        ;[1 0.6073 0.2872] Z rotation turret
        (if (not (== _returnvalue_2 (0.0 0.0 0.0)))
          (`self.setZworlLocation multi` (`self.turret_tray`) _get_base_position_roll _returnvalue_yaw_2)))
      (:`then_1`
        ;[1 0.8868 0.237] Y rotation turret
        (if (not (== _returnvalue (0.0 0.0 0.0)))
          (`self.setYWorldLocation multi` (`self.flameThrower_turret`) (+ _returnvalue_yaw_2 180.0) _returnvalue_pitch_3))))))

(event `setZworlLocation multi`
  (params (Target :type "SceneComponent Object Reference") (`New Rotation X (Roll)` :type "Float (double-precision)") (`New Rotation Z (Yaw)` :type "Float (double-precision)"))
  ;[1 0.6073 0.2872] Z rotation turret
  (`SceneComponent.K2_SetWorldRotation` Target (`KismetMathLibrary.MakeRotator` `New Rotation X (Roll)` 0.0 `New Rotation Z (Yaw)`) false false))

(event `setYWorldLocation multi`
  (params (Target :type "SceneComponent Object Reference") (`New Rotation Z (Yaw)` :type "Float (double-precision)") (`New Rotation Y (Pitch)` :type "Float (double-precision)"))
  ;[1 0.8868 0.237] Y rotation turret
  (`SceneComponent.K2_SetWorldRotation` Target (`KismetMathLibrary.MakeRotator` 0.0 `New Rotation Y (Pitch)` `New Rotation Z (Yaw)`) false false))

(event `fire action`
  ;[1 0 0.008842] fire action
  (if (`self.in range`)
    (if (== (`self.ammo`) 0)
      (`self.Stop Fire multi` :!label _label)
      (goto _label_2 :!via `Close`)
      (else
        (`|ExecutionSequence`
          (:`then_0`
            (`/Engine/EditorBlueprintResources/StandardMacros.Gate` true :!label _label_2
              (:`Exit`
                (`|ExecutionSequence`
                  (:`then_0`
                    (`KismetSystemLibrary.RetriggerableDelay` 0.2)
                    (goto _label_2))
                  (:`then_1`
                    (`KismetSystemLibrary.Delay` 0.2)
                    (set `self.ammo` (`KismetMathLibrary.Clamp` (- (`self.ammo`) 1) 0 (`self.max ammo`)))
                    (`self.fire multi` (`self.ammo`)))))))
          (:`then_1`
            (goto _label_2 :!via `Open`)))))
    (else
      (goto _label))))

(event `fire multi`
  (params (ammo :type Integer))
  ;[1 0 0.008842] fire action
  (`|ExecutionSequence`
    (:`then_0`
      (set `self.ammo` ammo)
      ;;[0.1586 1 0.1772] Custom Turret
      (`ActorComponent.Activate` (`self.ParticleSystem`) false))
    (:`then_1`
      (`/Engine/EditorBlueprintResources/StandardMacros.DoOnce` false :!label _label_3
        (:`Completed`
          (bind _returnvalue (`GameplayStatics.SpawnSound2D` "/Game/Automatic_FlameThrower_Turret/sounds/SC_flame_effect.SC_flame_effect"))
          (set `self.Flame Sound` _returnvalue))))))

(event `Stop Fire multi`
  (bind _flame_sound (`self.Flame Sound`))
  ;[1 0 0.008842] fire action
  (`|ExecutionSequence`
    (:`then_0`
      ;;[0.1586 1 0.1772] Custom Turret
      (`ActorComponent.Deactivate` (`self.ParticleSystem`)))
    (:`then_1`
      (`KismetSystemLibrary.Delay` 0.2)
      (`|ExecutionSequence`
        (:`then_0`
          (goto _label_3 :!via `Reset`))
        (:`then_1`
          (`/Engine/EditorBlueprintResources/StandardMacros.IsValid` _flame_sound
            (:`Is Valid`
              (`AudioComponent.FadeOut` _flame_sound 0.5 0.0))))))))

(event `self.Box.OnComponentBeginOverlap`
  (params (OverlappedComponent :type "PrimitiveComponent Object Reference") (OtherActor :type "Actor Object Reference") (OtherComp :type "PrimitiveComponent Object Reference") (OtherBodyIndex :type Integer) (bFromSweep :type Boolean) (SweepResult :type "HitResult Structure (by ref)"))
  (bind _returnvalue (and (not (`self.OFF`)) (`self.in range`)))
  ;[1 1 1] Get Target - set Target Fire - Apply damage
  (bind _ascharacter (cast `Character` OtherActor)
    (:`then`
      (if _returnvalue
        (set `self.Target hit?` true)
        (`GameplayStatics.SpawnEmitterAttached` "/Game/Automatic_FlameThrower_Turret/Particles/P_Fire_Player.P_Fire_Player" (`Actor.RootComponent` _ascharacter))
        (`|ExecutionSequence` :!label _label_4
          (:`then_0`
            (goto _label_5 :!via `Open`))
          (:`then_1`
            (`/Engine/EditorBlueprintResources/StandardMacros.Gate` true :!label _label_5
              (:`Exit`
                (`|ExecutionSequence`
                  (:`then_0`
                    (`KismetSystemLibrary.RetriggerableDelay` (`self.Rate of DMG`))
                    (goto _label_5))
                  (:`then_1`
                    (if (`self.Target hit?`)
                      (`KismetSystemLibrary.PrintString` "Hit"))))))))))
    (:`CastFailed`
      (bind _asbp_bot (cast `/Game/Automatic_FlameThrower_Turret/Character/NPC/BP_bot` OtherActor))
      (if _returnvalue
        (set `self.Target hit?` true)
        (`GameplayStatics.SpawnEmitterAttached` "/Game/Automatic_FlameThrower_Turret/Particles/P_Fire_Player.P_Fire_Player" (`Actor.RootComponent` _asbp_bot))
        (goto _label_4)))))

(event `self.Box.OnComponentEndOverlap`
  (params (OverlappedComponent :type "PrimitiveComponent Object Reference") (OtherActor :type "Actor Object Reference") (OtherComp :type "PrimitiveComponent Object Reference") (OtherBodyIndex :type Integer))
  ;[1 1 1] Get Target - set Target Fire - Apply damage
  (cast `Character` OtherActor
    (:`then`
      (set `self.Target hit?` false))
    (:`CastFailed`
      (cast `/Game/Automatic_FlameThrower_Turret/Character/NPC/BP_bot` OtherActor)
      (set `self.Target hit?` false))))

(fn `UserConstructionScript`)