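; BP_HoloPod is a sci-fi hologram pod prop that displays a configurable mesh as a rotating projection.
; When projecting, the construction script assigns the mesh, gives every slot a tinted dynamic material, colors the particles and lights the pod's top.
; Tick spins the mesh and rotates its relative location, so off-center meshes orbit the projector's origin.
; When off, construction destroys the projection components, applies an unlit display material and disables Tick.
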(event `self.ReceiveTick`
  (params (DeltaSeconds :type "Float (single-precision)"))
  (bind _returnvalue (* DeltaSeconds (`self.RotationSpeed`)))
  (if (`self.isProjecting`)
    ;[1 1 1] Rotate the mesh
    (`SceneComponent.K2_AddWorldRotation` (`self.ProjectedMesh`) (`KismetMathLibrary.MakeRotator` 0.0 0.0 _returnvalue) false false)
    ;[1 1 1] Move around the mesh if off-center so it still rotates around the projectors origin
    (`SceneComponent.K2_SetRelativeLocation` (`self.ProjectedMesh`) (`KismetMathLibrary.GreaterGreater_VectorRotator` (`SceneComponent.RelativeLocation` (`self.ProjectedMesh`)) (`KismetMathLibrary.MakeRotator` 0.0 0.0 _returnvalue)) false false)))

(fn `UserConstructionScript`
  (bind _projectedmesh (`self.ProjectedMesh`))
  (if (`self.isProjecting`)
    (`|ExecutionSequence`
      (:`then_0`
        ;[1 1 1] Set Up Projection Particles
        (`ParticleSystemComponent.SetVectorParameter` (`self.PS_Projection`) "Emissive_Color" (`KismetMathLibrary.Conv_LinearColorToVector` (`self.ProjectionColor`)))
        ;[1 1 1] Set up the projected mesh
        (`StaticMeshComponent.SetStaticMesh` _projectedmesh (`self.ProjectionMesh`))
        (for _index (range (`PrimitiveComponent.GetNumMaterials` _projectedmesh))
          (bind _returnvalue (`KismetMaterialLibrary.CreateDynamicMaterialInstance` (`self.ProjectionMaterial`)))
          (`MaterialInstanceDynamic.SetVectorParameterValue` _returnvalue "Emissive_Color" (`self.ProjectionColor`))
          (`PrimitiveComponent.SetMaterial` _projectedmesh _index _returnvalue)))
      (:`then_1`
        ;[1 1 1] Change the material on top
        (bind _returnvalue_2 (`KismetMaterialLibrary.CreateDynamicMaterialInstance` "/Game/Sci-fiCrimeScene/Materials/M_StrongGlow.M_StrongGlow"))
        (`PrimitiveComponent.SetMaterial` (`self.SM_Holopod`) 1 _returnvalue_2)
        (`MaterialInstanceDynamic.SetVectorParameterValue` _returnvalue_2 "Emissive_Color" (`self.TopEmissiveColor`))))
    (else
      ;[1 1 1] Delete projection dependent parts
      (`ActorComponent.K2_DestroyComponent` (`self.ProjectedMesh`))
      (`ActorComponent.K2_DestroyComponent` (`self.PS_Projection`))
      (`PrimitiveComponent.SetMaterial` (`self.SM_Holopod`) 1 "/Game/Sci-fiCrimeScene/Materials/Instances/Displays/MI_Display_off.MI_Display_off")
      (`self.SetActorTickEnabled` false))))