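; BP_PoliceDrone is a hovering sci-fi police drone with a colored projection and an optional spotlight.
; Each tick it bobs the Drone component on a sine wave around the Root and turns it toward the LookAt component.
; The construction script applies the projection color to the particles and a dynamic drone material.
; It also either sets the spotlight's intensity and brightness-normalized color, or destroys it when real lighting is off.
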(event `self.ReceiveTick`
  (params (DeltaSeconds :type "Float (single-precision)"))
  (bind _drone (`self.Drone`))
  (bind (_returnvalue_x _returnvalue_y _returnvalue_z) (`KismetMathLibrary.BreakVector` (`SceneComponent.K2_GetComponentLocation` (`self.Root`))))
  ;[1 1 1] Apply Changes
  (`SceneComponent.K2_SetWorldLocation` _drone (`KismetMathLibrary.MakeVector` _returnvalue_x _returnvalue_y (+ (* (`KismetMathLibrary.Sin` (* (`self.GetGameTimeSinceCreation`) (* (`self.HoverSpeed`) (`KismetMathLibrary.GetPI`)))) (`self.HoverAmount`)) _returnvalue_z)) false false)
  (`SceneComponent.K2_SetWorldRotation` _drone (`KismetMathLibrary.FindLookAtRotation` (`SceneComponent.K2_GetComponentLocation` (`self.Drone`)) (`SceneComponent.K2_GetComponentLocation` (`self.LookAt`))) false false))

(fn `getNormalizedColor`
  (returns (NormalizedColor :type "LinearColor Structure"))
  (bind _projectioncolor (`self.ProjectionColor`))
  (bind (_r _g _b) (`KismetMathLibrary.BreakColor` _projectioncolor))
  ;[1 1 1] calculate normalized color
  (return (* _projectioncolor (/ 1.0 (`KismetMathLibrary.FMax` _r _g _b)))))

(fn `UserConstructionScript`
  ;[1 1 1] Check if a real light is used
  (if (`self.UseRealLight`)
    ;[1 1 1] Set Light intensity and color
    (`LightComponent.SetLightColor` (`self.SpotLight`) (`self.getNormalizedColor`) true)
    (`LightComponent.SetIntensity` (`self.SpotLight`) (`self.LightIntensity`))
    (else
      ;[1 1 1] Delete light
      (`ActorComponent.K2_DestroyComponent` (`self.SpotLight`))))
  ;[1 1 1] set color of projection particles
  (`ParticleSystemComponent.SetVectorParameter` (`self.Projection`) "Emissive_Color" (`KismetMathLibrary.Conv_LinearColorToVector` (`self.ProjectionColor`)))
  ;[1 1 1] Set up new material instance to be used on the light
  (bind _returnvalue (`KismetMaterialLibrary.CreateDynamicMaterialInstance` (`self.Drone`) (`self.BaseInstance`)))
  (`MaterialInstanceDynamic.SetVectorParameterValue` _returnvalue "Emissive_Color" (`self.ProjectionColor`))
  (`PrimitiveComponent.SetMaterial` (`self.Drone`) 0 _returnvalue))