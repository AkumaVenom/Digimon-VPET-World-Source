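; Consumable DigiMeat inventory item that feeds the player's currently toggled Digimon pet.
; UseItem does nothing unless that pet is valid and its hunger is not above 99, then triggers its eat event and toggles the inventory.
; It adds a fixed hunger amount by rebuilding the whole PetStructure, clamps it to a hardcoded 100 rather than MaxHunger, fires the pet's poop event and returns true.
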(fn `UseItem`
  (returns (Success :type Boolean))
  (`parent.UseItem`)
  (bind _asmaster_character_bp (cast `/Game/MAIN/Blueprints/Player/MasterCharacter_BP` (`GameplayStatics.GetPlayerCharacter` 0)))
  (bind _toggledpet (`/Game/MAIN/Blueprints/Player/MasterCharacter_BP.ToggledPet` _asmaster_character_bp)
    (:`then`
      (bind (_petstructure_name _petstructure_isstackable _petstructure_thumbnail _petstructure_maxstacksize _petstructure_isconsumable _petstructure_description _petstructure_class _petstructure_pettag _petstructure_pettype _petstructure_raretype _petstructure_mood _petstructure_trait _petstructure_ispetforquest _petstructure_trainerownedby _petstructure_cost _petstructure_level _petstructure_currenthealth _petstructure_maxhealth _petstructure_mindamage _petstructure_maxdamage _petstructure_currentmana _petstructure_maxmana _petstructure_isownedbyplayer _petstructure_isdead _petstructure_issummoned _petstructure_iswild _petstructure_isattacking _petstructure_isusingability1 _petstructure_isusingability2 _petstructure_isusingability3 _petstructure_isusingability4 _petstructure_isshiny _petstructure_petsize _petstructure_abi _petstructure_def _petstructure_int _petstructure_spd _petstructure_vpettype _petstructure_vpetattribute _petstructure_digivolve1 _petstructure_digivolve2 _petstructure_digivolve3 _petstructure_digivolve4 _petstructure_digivolve5 _petstructure_digivolve6 _petstructure_digivolve7 _petstructure_digivolve8 _petstructure_digivolve9 _petstructure_digivolve10 _petstructure_digivolve11 _petstructure_digivolve12 _petstructure_isstarterdigimon _petstructure_candigivolve1 _petstructure_candigivolve2 _petstructure_candigivolve3 _petstructure_candigivolve4 _petstructure_candigivolve5 _petstructure_candigivolve6 _petstructure_candigivolve7 _petstructure_candigivolve8 _petstructure_candigivolve9 _petstructure_candigivolve10 _petstructure_candigivolve11 _petstructure_candigivolve12 _petstructure_diddigivolve1 _petstructure_diddigivolve2 _petstructure_diddigivolve3 _petstructure_diddigivolve4 _petstructure_diddigivolve5 _petstructure_diddigivolve6 _petstructure_diddigivolve7 _petstructure_diddigivolve8 _petstructure_diddigivolve9 _petstructure_diddigivolve10 _petstructure_diddigivolve11 _petstructure_diddigivolve12 _petstructure_dedigivolve1 _petstructure_dedigivolve2 _petstructure_dedigivolve3 _petstructure_dedigivolve4 _petstructure_dedigivolve5 _petstructure_dedigivolve6 _petstructure_dedigivolve7 _petstructure_dedigivolve8 _petstructure_dedigivolve9 _petstructure_dedigivolve10 _petstructure_dedigivolve11 _petstructure_dedigivolve12 _petstructure_candedigivolve1 _petstructure_candedigivolve2 _petstructure_candedigivolve3 _petstructure_candedigivolve4 _petstructure_candedigivolve5 _petstructure_candedigivolve6 _petstructure_candedigivolve7 _petstructure_candedigivolve8 _petstructure_candedigivolve9 _petstructure_candedigivolve10 _petstructure_candedigivolve11 _petstructure_candedigivolve12 _petstructure_diddedigivolve1 _petstructure_diddedigivolve2 _petstructure_diddedigivolve3 _petstructure_diddedigivolve4 _petstructure_diddedigivolve5 _petstructure_diddedigivolve6 _petstructure_diddedigivolve7 _petstructure_diddedigivolve8 _petstructure_diddedigivolve9 _petstructure_diddedigivolve10 _petstructure_diddedigivolve11 _petstructure_diddedigivolve12 _petstructure_leveltype _petstructure_ishostile _petstructure_currentxp _petstructure_neededxp _petstructure_currenthunger _petstructure_maxhunger) (break `/Game/MAIN/PetSystem/DigimonVPetsStructure` (`/Game/MAIN/PetSystem/Pets/Parent/Pet_Parent_BP.PetStructure` _toggledpet)))
      (if (not (> _petstructure_currenthunger 99))
        (`/Game/MAIN/PetSystem/Pets/Parent/Pet_Parent_BP.EatFoodEvent` _toggledpet)
        (`/Game/MAIN/InventorySystem/InventoryComponent.ToggleInventory` (`/Game/MAIN/Blueprints/Player/MasterCharacter_BP.InventoryComponent` _asmaster_character_bp))
        (`|ExecutionSequence`
          (:`then_1`
            (bind _output_get (set `/Game/MAIN/PetSystem/Pets/Parent/Pet_Parent_BP.PetStructure` (make `/Game/MAIN/PetSystem/DigimonVPetsStructure` _petstructure_name _petstructure_isstackable _petstructure_thumbnail _petstructure_maxstacksize _petstructure_isconsumable _petstructure_description _petstructure_class _petstructure_pettag _petstructure_pettype _petstructure_raretype _petstructure_mood _petstructure_trait _petstructure_ispetforquest _petstructure_trainerownedby _petstructure_cost _petstructure_level _petstructure_currenthealth _petstructure_maxhealth _petstructure_mindamage _petstructure_maxdamage _petstructure_currentmana _petstructure_maxmana _petstructure_isownedbyplayer _petstructure_isdead _petstructure_issummoned _petstructure_iswild _petstructure_isattacking _petstructure_isusingability1 _petstructure_isusingability2 _petstructure_isusingability3 _petstructure_isusingability4 _petstructure_isshiny _petstructure_petsize _petstructure_abi _petstructure_def _petstructure_int _petstructure_spd _petstructure_vpettype _petstructure_vpetattribute _petstructure_digivolve1 _petstructure_digivolve2 _petstructure_digivolve3 _petstructure_digivolve4 _petstructure_digivolve5 _petstructure_digivolve6 _petstructure_digivolve7 _petstructure_digivolve8 _petstructure_digivolve9 _petstructure_digivolve10 _petstructure_digivolve11 _petstructure_digivolve12 _petstructure_isstarterdigimon _petstructure_candigivolve1 _petstructure_candigivolve2 _petstructure_candigivolve3 _petstructure_candigivolve4 _petstructure_candigivolve5 _petstructure_candigivolve6 _petstructure_candigivolve7 _petstructure_candigivolve8 _petstructure_candigivolve9 _petstructure_candigivolve10 _petstructure_candigivolve11 _petstructure_candigivolve12 _petstructure_diddigivolve1 _petstructure_diddigivolve2 _petstructure_diddigivolve3 _petstructure_diddigivolve4 _petstructure_diddigivolve5 _petstructure_diddigivolve6 _petstructure_diddigivolve7 _petstructure_diddigivolve8 _petstructure_diddigivolve9 _petstructure_diddigivolve10 _petstructure_diddigivolve11 _petstructure_diddigivolve12 _petstructure_dedigivolve1 _petstructure_dedigivolve2 _petstructure_dedigivolve3 _petstructure_dedigivolve4 _petstructure_dedigivolve5 _petstructure_dedigivolve6 _petstructure_dedigivolve7 _petstructure_dedigivolve8 _petstructure_dedigivolve9 _petstructure_dedigivolve10 _petstructure_dedigivolve11 _petstructure_dedigivolve12 _petstructure_candedigivolve1 _petstructure_candedigivolve2 _petstructure_candedigivolve3 _petstructure_candedigivolve4 _petstructure_candedigivolve5 _petstructure_candedigivolve6 _petstructure_candedigivolve7 _petstructure_candedigivolve8 _petstructure_candedigivolve9 _petstructure_candedigivolve10 _petstructure_candedigivolve11 _petstructure_candedigivolve12 _petstructure_diddedigivolve1 _petstructure_diddedigivolve2 _petstructure_diddedigivolve3 _petstructure_diddedigivolve4 _petstructure_diddedigivolve5 _petstructure_diddedigivolve6 _petstructure_diddedigivolve7 _petstructure_diddedigivolve8 _petstructure_diddedigivolve9 _petstructure_diddedigivolve10 _petstructure_diddedigivolve11 _petstructure_diddedigivolve12 _petstructure_leveltype _petstructure_ishostile _petstructure_currentxp _petstructure_neededxp (+ _petstructure_currenthunger 30) _petstructure_maxhunger) _toggledpet))
            (if (> (`.CurrentHunger_285_A193949949ABBEF6E2D60FB884C8CC66` (break `/Game/MAIN/PetSystem/DigimonVPetsStructure` _output_get)) 99)
              (bind (_petstructure_name_2 _petstructure_isstackable_2 _petstructure_thumbnail_2 _petstructure_maxstacksize_2 _petstructure_isconsumable_2 _petstructure_description_2 _petstructure_class_2 _petstructure_pettag_2 _petstructure_pettype_2 _petstructure_raretype_2 _petstructure_mood_2 _petstructure_trait_2 _petstructure_ispetforquest_2 _petstructure_trainerownedby_2 _petstructure_cost_2 _petstructure_level_2 _petstructure_currenthealth_2 _petstructure_maxhealth_2 _petstructure_mindamage_2 _petstructure_maxdamage_2 _petstructure_currentmana_2 _petstructure_maxmana_2 _petstructure_isownedbyplayer_2 _petstructure_isdead_2 _petstructure_issummoned_2 _petstructure_iswild_2 _petstructure_isattacking_2 _petstructure_isusingability1_2 _petstructure_isusingability2_2 _petstructure_isusingability3_2 _petstructure_isusingability4_2 _petstructure_isshiny_2 _petstructure_petsize_2 _petstructure_abi_2 _petstructure_def_2 _petstructure_int_2 _petstructure_spd_2 _petstructure_vpettype_2 _petstructure_vpetattribute_2 _petstructure_digivolve1_2 _petstructure_digivolve2_2 _petstructure_digivolve3_2 _petstructure_digivolve4_2 _petstructure_digivolve5_2 _petstructure_digivolve6_2 _petstructure_digivolve7_2 _petstructure_digivolve8_2 _petstructure_digivolve9_2 _petstructure_digivolve10_2 _petstructure_digivolve11_2 _petstructure_digivolve12_2 _petstructure_isstarterdigimon_2 _petstructure_candigivolve1_2 _petstructure_candigivolve2_2 _petstructure_candigivolve3_2 _petstructure_candigivolve4_2 _petstructure_candigivolve5_2 _petstructure_candigivolve6_2 _petstructure_candigivolve7_2 _petstructure_candigivolve8_2 _petstructure_candigivolve9_2 _petstructure_candigivolve10_2 _petstructure_candigivolve11_2 _petstructure_candigivolve12_2 _petstructure_diddigivolve1_2 _petstructure_diddigivolve2_2 _petstructure_diddigivolve3_2 _petstructure_diddigivolve4_2 _petstructure_diddigivolve5_2 _petstructure_diddigivolve6_2 _petstructure_diddigivolve7_2 _petstructure_diddigivolve8_2 _petstructure_diddigivolve9_2 _petstructure_diddigivolve10_2 _petstructure_diddigivolve11_2 _petstructure_diddigivolve12_2 _petstructure_dedigivolve1_2 _petstructure_dedigivolve2_2 _petstructure_dedigivolve3_2 _petstructure_dedigivolve4_2 _petstructure_dedigivolve5_2 _petstructure_dedigivolve6_2 _petstructure_dedigivolve7_2 _petstructure_dedigivolve8_2 _petstructure_dedigivolve9_2 _petstructure_dedigivolve10_2 _petstructure_dedigivolve11_2 _petstructure_dedigivolve12_2 _petstructure_candedigivolve1_2 _petstructure_candedigivolve2_2 _petstructure_candedigivolve3_2 _petstructure_candedigivolve4_2 _petstructure_candedigivolve5_2 _petstructure_candedigivolve6_2 _petstructure_candedigivolve7_2 _petstructure_candedigivolve8_2 _petstructure_candedigivolve9_2 _petstructure_candedigivolve10_2 _petstructure_candedigivolve11_2 _petstructure_candedigivolve12_2 _petstructure_diddedigivolve1_2 _petstructure_diddedigivolve2_2 _petstructure_diddedigivolve3_2 _petstructure_diddedigivolve4_2 _petstructure_diddedigivolve5_2 _petstructure_diddedigivolve6_2 _petstructure_diddedigivolve7_2 _petstructure_diddedigivolve8_2 _petstructure_diddedigivolve9_2 _petstructure_diddedigivolve10_2 _petstructure_diddedigivolve11_2 _petstructure_diddedigivolve12_2 _petstructure_leveltype_2 _petstructure_ishostile_2 _petstructure_currentxp_2 _petstructure_neededxp_2 _petstructure_currenthunger_2 _petstructure_maxhunger_2) (break `/Game/MAIN/PetSystem/DigimonVPetsStructure` (`/Game/MAIN/PetSystem/Pets/Parent/Pet_Parent_BP.PetStructure` _toggledpet)))
              (set `/Game/MAIN/PetSystem/Pets/Parent/Pet_Parent_BP.PetStructure` (make `/Game/MAIN/PetSystem/DigimonVPetsStructure` _petstructure_name_2 _petstructure_isstackable_2 _petstructure_thumbnail_2 _petstructure_maxstacksize_2 _petstructure_isconsumable_2 _petstructure_description_2 _petstructure_class_2 _petstructure_pettag_2 _petstructure_pettype_2 _petstructure_raretype_2 _petstructure_mood_2 _petstructure_trait_2 _petstructure_ispetforquest_2 _petstructure_trainerownedby_2 _petstructure_cost_2 _petstructure_level_2 _petstructure_currenthealth_2 _petstructure_maxhealth_2 _petstructure_mindamage_2 _petstructure_maxdamage_2 _petstructure_currentmana_2 _petstructure_maxmana_2 _petstructure_isownedbyplayer_2 _petstructure_isdead_2 _petstructure_issummoned_2 _petstructure_iswild_2 _petstructure_isattacking_2 _petstructure_isusingability1_2 _petstructure_isusingability2_2 _petstructure_isusingability3_2 _petstructure_isusingability4_2 _petstructure_isshiny_2 _petstructure_petsize_2 _petstructure_abi_2 _petstructure_def_2 _petstructure_int_2 _petstructure_spd_2 _petstructure_vpettype_2 _petstructure_vpetattribute_2 _petstructure_digivolve1_2 _petstructure_digivolve2_2 _petstructure_digivolve3_2 _petstructure_digivolve4_2 _petstructure_digivolve5_2 _petstructure_digivolve6_2 _petstructure_digivolve7_2 _petstructure_digivolve8_2 _petstructure_digivolve9_2 _petstructure_digivolve10_2 _petstructure_digivolve11_2 _petstructure_digivolve12_2 _petstructure_isstarterdigimon_2 _petstructure_candigivolve1_2 _petstructure_candigivolve2_2 _petstructure_candigivolve3_2 _petstructure_candigivolve4_2 _petstructure_candigivolve5_2 _petstructure_candigivolve6_2 _petstructure_candigivolve7_2 _petstructure_candigivolve8_2 _petstructure_candigivolve9_2 _petstructure_candigivolve10_2 _petstructure_candigivolve11_2 _petstructure_candigivolve12_2 _petstructure_diddigivolve1_2 _petstructure_diddigivolve2_2 _petstructure_diddigivolve3_2 _petstructure_diddigivolve4_2 _petstructure_diddigivolve5_2 _petstructure_diddigivolve6_2 _petstructure_diddigivolve7_2 _petstructure_diddigivolve8_2 _petstructure_diddigivolve9_2 _petstructure_diddigivolve10_2 _petstructure_diddigivolve11_2 _petstructure_diddigivolve12_2 _petstructure_dedigivolve1_2 _petstructure_dedigivolve2_2 _petstructure_dedigivolve3_2 _petstructure_dedigivolve4_2 _petstructure_dedigivolve5_2 _petstructure_dedigivolve6_2 _petstructure_dedigivolve7_2 _petstructure_dedigivolve8_2 _petstructure_dedigivolve9_2 _petstructure_dedigivolve10_2 _petstructure_dedigivolve11_2 _petstructure_dedigivolve12_2 _petstructure_candedigivolve1_2 _petstructure_candedigivolve2_2 _petstructure_candedigivolve3_2 _petstructure_candedigivolve4_2 _petstructure_candedigivolve5_2 _petstructure_candedigivolve6_2 _petstructure_candedigivolve7_2 _petstructure_candedigivolve8_2 _petstructure_candedigivolve9_2 _petstructure_candedigivolve10_2 _petstructure_candedigivolve11_2 _petstructure_candedigivolve12_2 _petstructure_diddedigivolve1_2 _petstructure_diddedigivolve2_2 _petstructure_diddedigivolve3_2 _petstructure_diddedigivolve4_2 _petstructure_diddedigivolve5_2 _petstructure_diddedigivolve6_2 _petstructure_diddedigivolve7_2 _petstructure_diddedigivolve8_2 _petstructure_diddedigivolve9_2 _petstructure_diddedigivolve10_2 _petstructure_diddedigivolve11_2 _petstructure_diddedigivolve12_2 _petstructure_leveltype_2 _petstructure_ishostile_2 _petstructure_currentxp_2 _petstructure_neededxp_2 100 _petstructure_maxhunger_2) _toggledpet)
              (`/Game/MAIN/PetSystem/Pets/Parent/Pet_Parent_BP.PoopEvent` _toggledpet)
              (return true)
              (else
                (`/Game/MAIN/PetSystem/Pets/Parent/Pet_Parent_BP.PoopEvent` _toggledpet)
                (return true)))))))
    (:`else`)))

(fn `UserConstructionScript`
  (`parent.UserConstructionScript`))