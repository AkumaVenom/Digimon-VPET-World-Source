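; Base Blueprint for world item pickups, with a stub UseItem that returns false.
; Visual components have collision disabled, and the paper sprite yaws toward the player every tick.
; Interact picks up normal items directly, but quest items only when their class matches a quest objective's target.
; A one-shot pickup adds the item to the player's inventory, then on success notifies incomplete quests and destroys the actor after a brief delay.
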(event `self.ReceiveBeginPlay`
  (bind _asmaster_character_bp (cast `/Game/MAIN/Blueprints/Player/MasterCharacter_BP` (`GameplayStatics.GetPlayerCharacter` 0)))
  (set `self.PlayerReference` _asmaster_character_bp)
  (`PrimitiveComponent.SetCollisionEnabled` (`self.PaperSprite`) "NoCollision")
  (`PrimitiveComponent.SetCollisionEnabled` (`self.StaticMesh`) "NoCollision")
  (`PrimitiveComponent.SetCollisionEnabled` (`self.SkeletalMesh`) "NoCollision")
  (`PrimitiveComponent.SetCollisionEnabled` (`self.ParticleSystem`) "NoCollision"))

(event `self.ReceiveTick`
  (params (DeltaSeconds :type "Float (single-precision)"))
  (`self.FacePlayer`))

(event `self.ReceiveActorBeginOverlap`
  (params (OtherActor :type "Actor Object Reference"))
  (if true
    _))

(event `/Game/MAIN/QuestSystem/InteractInterface.Interact`
  (params (Interacter :type "Actor Object Reference"))
  (bind (_itemstructure_name _itemstructure_isstackable _itemstructure_thumbnail _itemstructure_description _itemstructure_isconsumable _itemstructure_maxstacksize _itemstructure_durability _itemstructure_class _itemstructure_isquestitem) (break `/Game/MAIN/InventorySystem/ItemStructure` (`self.ItemStructure`)))
  (if _itemstructure_isquestitem
    (bind _asmaster_character_bp (cast `/Game/MAIN/Blueprints/Player/MasterCharacter_BP` (`GameplayStatics.GetPlayerCharacter` 0)))
    (for _array_element (`/Game/MAIN/QuestSystem/QuestLog.Quests` (`/Game/MAIN/Blueprints/Player/MasterCharacter_BP.QuestLog` _asmaster_character_bp))
      (for _array_element_2 (`/Game/MAIN/QuestSystem/Quests/QuestMaster_BP.Objectives` _array_element)
        (if (== (`GameplayStatics.GetObjectClass` (`.Target_11_8F5BC56B4D2EF62A87A2D285AE43AC8A` (break `/Game/MAIN/QuestSystem/Objectives/ObjectiveData` _array_element_2))) (`GameplayStatics.GetObjectClass` self))
          (`self.PickupItem`))))
    (else
      (`self.PickupItem`))))

(event `PickupItem`
  (`/Engine/EditorBlueprintResources/StandardMacros.DoOnce` false
    (:`Completed`
      (bind _asmaster_character_bp (cast `/Game/MAIN/Blueprints/Player/MasterCharacter_BP` (`GameplayStatics.GetPlayerCharacter` 0)))
      (bind _success (`/Game/MAIN/InventorySystem/InventoryComponent.AddToInventory` (`/Game/MAIN/Blueprints/Player/MasterCharacter_BP.InventoryComponent` _asmaster_character_bp) (make `/Game/MAIN/InventorySystem/SlotStructure` (`self.ItemStructure`) 1)))
      (if _success
        (`|ExecutionSequence`
          (:`then_0`
            (`KismetSystemLibrary.Delay` 0.2)
            (`/Engine/EditorBlueprintResources/StandardMacros.IsValid` self
              (:`Is Valid`
                (`self.K2_DestroyActor`))))
          (:`then_1`
            (for _array_element (`/Game/MAIN/QuestSystem/QuestLog.Quests` (`/Game/MAIN/Blueprints/Player/MasterCharacter_BP.QuestLog` _asmaster_character_bp))
              (if (not (`/Game/MAIN/QuestSystem/Quests/QuestMaster_BP.IsComplete` _array_element))
                (`/Game/MAIN/QuestSystem/Quests/QuestMaster_BP.CollectedItem` _array_element self)))))))))

(fn `FacePlayer`
  (bind _papersprite (`self.PaperSprite`))
  (bind _playerreference (`self.PlayerReference`)
    (:`then`
      (bind (_returnvalue_roll _returnvalue_pitch _returnvalue_yaw) (`KismetMathLibrary.BreakRotator` (`KismetMathLibrary.FindLookAtRotation` (`SceneComponent.K2_GetComponentLocation` _papersprite) (`self.K2_GetActorLocation` _playerreference))))
      (`SceneComponent.K2_SetWorldRotation` _papersprite (`KismetMathLibrary.MakeRotator` 0.0 0.0 (- _returnvalue_yaw 90.0)) false false)
      (return))
    (:`else`)))

(fn `UseItem`
  (returns (Success :type Boolean))
  (return false))

(fn `UserConstructionScript`)