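; Base Blueprint for world containers that hold items and open their inventory when a character interacts with them.
; On BeginPlay it copies each entry of its Items array into the matching slot of its InventoryComponent's inventory.
; Interact toggles that inventory component only when the interacter is a MasterCharacter_BP.
; Overlap and Tick events only print empty strings.
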(event `self.ReceiveActorBeginOverlap`
  (params (OtherActor :type "Actor Object Reference"))
  (`KismetSystemLibrary.PrintString` " "))

(event `self.ReceiveTick`
  (params (DeltaSeconds :type "Float (single-precision)"))
  (`KismetSystemLibrary.PrintString` " "))

(event `self.ReceiveBeginPlay`
  (for (_array_element _array_index) (`self.Items`)
    (`KismetArrayLibrary.Array_Set` (`/Game/MAIN/InventorySystem/InventoryComponent.Inventory` (`self.InventoryComponent`)) _array_index _array_element)))

(event `/Game/MAIN/QuestSystem/InteractInterface.Interact`
  (params (Interacter :type "Actor Object Reference"))
  (cast `/Game/MAIN/Blueprints/Player/MasterCharacter_BP` Interacter)
  (`/Game/MAIN/InventorySystem/InventoryComponent.ToggleInventory` (`self.InventoryComponent`)))

(fn `UserConstructionScript`)