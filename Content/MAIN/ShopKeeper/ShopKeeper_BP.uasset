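; ShopKeeper_BP is a shopkeeper NPC that opens a shop screen when the player interacts with it.
; Interact blends the camera to the shopkeeper, shows the mouse cursor, stops and disables the MasterCharacter_BP player's movement, and hides that character.
; It flags the player as in the shop, then after a short delay matching the blend creates ShopKeeper_UI with a reference to itself and adds it to the viewport.
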(event `/Game/MAIN/QuestSystem/InteractInterface.Interact`
  (params (Interacter :type "Actor Object Reference"))
  (`PlayerController.SetViewTargetWithBlend` (`GameplayStatics.GetPlayerController` 0) self 1.0 "VTBlend_Linear" 0.0 false)
  (set `PlayerController.bShowMouseCursor` true (`GameplayStatics.GetPlayerController` 0))
  (bind _asmaster_character_bp (cast `/Game/MAIN/Blueprints/Player/MasterCharacter_BP` (`GameplayStatics.GetPlayerCharacter` 0)))
  (bind _charactermovement (`Character.CharacterMovement` _asmaster_character_bp))
  (`CharacterMovementComponent.DisableMovement` _charactermovement)
  (`MovementComponent.StopMovementImmediately` _charactermovement)
  (`self.SetActorHiddenInGame` _asmaster_character_bp true)
  (set `self.PlayerIsInShop` true)
  (`KismetSystemLibrary.Delay` 1.0)
  (bind _returnvalue (`|CreateWidget` "/Game/MAIN/ShopKeeper/UI/ShopKeeper_UI.ShopKeeper_UI_C" null self))
  (`UserWidget.AddToViewport` _returnvalue 0))

(fn `UserConstructionScript`)