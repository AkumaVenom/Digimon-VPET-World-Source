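; Parent Blueprint for sprite-based NPCs that can roam, turn hostile and open their inventory on interaction when dead.
; Tick yaws the Paper sprite toward the player, alternates leg sprites while moving, loops random roaming and destroys distant NPCs.
; Pawn sensing starts looping AIMoveTo chases: melee damages the player and flashes a wound widget, while ranged repositions nearby and only plays an attack pose.
; DeathEvent and CalculateLoot are empty stubs.
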(event `/Game/MAIN/QuestSystem/InteractInterface.Interact`
  (params (Interacter :type "Actor Object Reference"))
  (cast `/Game/MAIN/Blueprints/Player/MasterCharacter_BP` Interacter)
  (if (<= (`self.CurrentHealth`) 0)
    (`/Game/MAIN/InventorySystem/InventoryComponent.ToggleInventory` (`self.InventoryComponent`))))

(event `self.ReceiveBeginPlay`
  (bind _asmaster_character_bp (cast `/Game/MAIN/Blueprints/Player/MasterCharacter_BP` (`GameplayStatics.GetPlayerCharacter` 0)))
  (set `self.PlayerReference` _asmaster_character_bp)
  (`self.CalculateLoot`))

(event `self.ReceiveTick`
  (params (DeltaSeconds :type "Float (single-precision)"))
  (bind _idlesprite (`self.IdleSprite`))
  (`|ExecutionSequence`
    (:`then_0`
      (if (> (`self.GetDistanceTo` self (`self.PlayerReference`)) (`self.RadiusToDespawn`))
        (`/Engine/EditorBlueprintResources/StandardMacros.DoOnce` false
          (:`Completed`
            (`self.K2_DestroyActor`)))))
    (:`then_1`
      (`self.FacePlayer`))
    (:`then_2`
      (if (> (`KismetMathLibrary.VSize` (`self.GetVelocity`)) 0.1)
        (if (or (`self.IsMeleeEnemy`) (`self.IsRangedEnemy`))
          (`/Engine/EditorBlueprintResources/StandardMacros.DoOnce` false :!label _label
            (:`Completed`
              (`/Engine/EditorBlueprintResources/StandardMacros.FlipFlop`
                (:`A`
                  (`PaperSpriteComponent.SetSprite` (`self.PaperSprite`) (`self.LLegSprite`))
                  (`KismetSystemLibrary.Delay` 0.2)
                  (`PaperSpriteComponent.SetSprite` (`self.PaperSprite`) _idlesprite)
                  (goto _label :!via `Reset`))
                (:`B`
                  (`PaperSpriteComponent.SetSprite` (`self.PaperSprite`) (`self.RLegSprite`))
                  (`KismetSystemLibrary.Delay` 0.2)
                  (`PaperSpriteComponent.SetSprite` (`self.PaperSprite`) _idlesprite)
                  (goto _label :!via `Reset`))))))))
    (:`then_3`
      (if (`self.CanFreeRoam`)
        (`KismetSystemLibrary.Delay` (`KismetMathLibrary.RandomFloatInRange` 3.0 7.0))
        (set `CharacterMovementComponent.MaxWalkSpeed` (`self.MaxWalkSpeedFreeRoam`) (`self.CharacterMovement`))
        (set `self.IsMoving` true)
        (`|AIMoveTo` self (`NavigationSystemV1.K2_GetRandomReachablePointInRadius` (`self.K2_GetActorLocation`) 2000.0 null null) null
          (:`OnSuccess`
            _)
          (:`OnFail`
            _))
        (set `self.IsMoving` false)))))

(event `DeathEvent`)

(event `self.PawnSensing.OnSeePawn`
  (params (Pawn :type "Pawn Object Reference"))
  (cast `/Game/MAIN/Blueprints/Player/MasterCharacter_BP` Pawn)
  (bind _playerreference (`self.PlayerReference` :!label _label_2)
    (:`then`
      (if (`self.IsHostile`)
        (if (`self.IsDead`)
          _
          (elif (`self.IsMeleeEnemy`)
            (`|AIMoveTo` self (0.0 0.0 0.0) _playerreference 100.0 :!label _label_3
              (:`then`
                (`KismetSystemLibrary.Delay` 1.0)
                (if (not (`self.IsDead`))
                  (goto _label_3)))
              (:`OnSuccess`
                (if (`self.CanAttack`)
                  (set `self.CanAttack` false)
                  (`PaperSpriteComponent.SetSprite` (`self.PaperSprite`) (`self.MeleeAttackSprite1`))
                  (set `self.IsAttacking` true)
                  (`KismetSystemLibrary.Delay` 0.2)
                  (`PaperSpriteComponent.SetSprite` (`self.PaperSprite`) (`self.MeleeAttackSprite2`))
                  (`self.WoundUI`
                    (:`then`
                      _)
                    (:`else`
                      (bind _returnvalue (`|CreateWidget` "/Game/MAIN/UI/Wound_UI.Wound_UI_C"))
                      (bind _output_get (set `self.WoundUI` _returnvalue))
                      (`UserWidget.AddToViewport` _output_get 0)))
                  (`|ExecutionSequence`
                    (:`then_0`
                      (`KismetSystemLibrary.Delay` 0.2)
                      (`PaperSpriteComponent.SetSprite` (`self.PaperSprite`) (`self.MeleeIdle`)))
                    (:`then_1`
                      (`KismetSystemLibrary.Delay` 0.7)
                      (set `self.CanAttack` true)
                      (set `self.IsAttacking` false)
                      (bind _woundui (`self.WoundUI`)
                        (:`then`
                          (`Widget.RemoveFromParent` _woundui))
                        (:`else`
                          _))
                      (set `self.WoundUI` null))
                    (:`then_2`
                      (bind _playerreference_2 (`self.PlayerReference`)
                        (:`then`
                          (bind _output_get_2 (set `/Game/MAIN/Blueprints/Player/MasterCharacter_BP.CurrentHealth` (- (`/Game/MAIN/Blueprints/Player/MasterCharacter_BP.CurrentHealth` _playerreference_2) (`self.DMG`)) _playerreference_2))
                          (if (< _output_get_2 1)
                            (set `/Game/MAIN/Blueprints/Player/MasterCharacter_BP.CurrentHealth` 0 _playerreference_2)
                            (`/Engine/EditorBlueprintResources/StandardMacros.DoOnce` false)))
                        (:`else`))))))
              (:`OnFail`
                (`KismetSystemLibrary.Delay` 0.2)
                (goto _label_2)))
            (elif (`self.IsRangedEnemy`)
              (bind _playerreference_3 (`self.PlayerReference` :!label _label_4)
                (:`then`
                  (`|AIMoveTo` self (`NavigationSystemV1.K2_GetRandomReachablePointInRadius` (`self.K2_GetActorLocation` _playerreference_3) 1000.0 null null) null 800.0
                    (:`then`
                      (`KismetSystemLibrary.Delay` 4.0 :!label _label_5)
                      (if (not (`self.IsDead`))
                        (goto _label_4)))
                    (:`OnSuccess`
                      (`|ExecutionSequence`
                        (:`then_0`
                          (goto _label_5))
                        (:`then_1`
                          (`/Engine/EditorBlueprintResources/StandardMacros.DoOnce` false :!label _label_6
                            (:`Completed`
                              (set `self.IsAttacking` true)
                              (`PaperSpriteComponent.SetSprite` (`self.PaperSprite`) (`self.MeleeAttackSprite1`))
                              (`KismetSystemLibrary.Delay` 1.0)
                              (set `self.IsAttacking` false))))
                        (:`then_2`
                          (`KismetSystemLibrary.Delay` (`KismetMathLibrary.RandomFloatInRange` 1.0 3.0))
                          (goto _label_6 :!via `Reset`))))
                    (:`OnFail`
                      (`KismetSystemLibrary.Delay` 0.2)
                      (goto _label_5))))
                (:`else`)))))))
    (:`else`)))

(event `self.PawnSensing.OnHearNoise`
  (params (Instigator :type "Pawn Object Reference") (Location :type "Vector Structure (by ref)") (Volume :type "Float (single-precision)"))
  (cast `/Game/MAIN/Blueprints/Player/MasterCharacter_BP` Instigator)
  (goto _label_2))

(fn `CalculateLoot`)

(fn `FacePlayer`
  (bind _papersprite (`self.PaperSprite`))
  (bind _playerreference (`self.PlayerReference`)
    (:`then`
      (`/Engine/EditorBlueprintResources/StandardMacros.IsValid` self
        (:`Is Valid`
          (bind (_returnvalue_roll _returnvalue_pitch _returnvalue_yaw) (`KismetMathLibrary.BreakRotator` (`KismetMathLibrary.FindLookAtRotation` (`SceneComponent.K2_GetComponentLocation` _papersprite) (`self.K2_GetActorLocation` _playerreference))))
          (`SceneComponent.K2_SetWorldRotation` _papersprite (`KismetMathLibrary.MakeRotator` 0.0 0.0 (- _returnvalue_yaw 90.0)) false false)
          (return))))
    (:`else`)))

(fn `UserConstructionScript`)