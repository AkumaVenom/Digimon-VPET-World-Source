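; Interactable Digi World PC that sends the player to the OpenWorldMap level once they have picked a starter Digimon.
; On Interact, it checks the interacting MasterCharacter_BP's starter flag, then saves player character 0's variables and opens the map after a short delay.
; Without a starter, it replaces any existing prompt with a DisplayTextUI widget telling the player to pick one first.
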(event `/Game/MAIN/QuestSystem/InteractInterface.Interact`
  (params (Interacter :type "Actor Object Reference"))
  (bind _asmaster_character_bp (cast `/Game/MAIN/Blueprints/Player/MasterCharacter_BP` Interacter))
  (if (`/Game/MAIN/Blueprints/Player/MasterCharacter_BP.StarterDigimonPicked` _asmaster_character_bp)
    (bind _asmaster_character_bp_2 (cast `/Game/MAIN/Blueprints/Player/MasterCharacter_BP` (`GameplayStatics.GetPlayerCharacter` 0)))
    (`/Game/MAIN/Blueprints/Player/MasterCharacter_BP.SavePlayerVaribles` _asmaster_character_bp_2)
    (`KismetSystemLibrary.Delay` 4.0)
    (`GameplayStatics.OpenLevel` "OpenWorldMap" false)
    (else
      (bind _pickstarterui (`self.PickStarterUI`)
        (:`then`
          (`Widget.RemoveFromParent` _pickstarterui))
        (:`else`
          _))
      (set `self.PickStarterUI` null)
      (bind _returnvalue (`|CreateWidget` "/Game/MAIN/UI/DisplayTextUI.DisplayTextUI_C" null "Pick a starter digimon first."))
      (bind _output_get (set `self.PickStarterUI` _returnvalue))
      (`UserWidget.AddToViewport` _output_get 0))))

(fn `UserConstructionScript`)