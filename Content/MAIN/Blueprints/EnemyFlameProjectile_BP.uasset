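; Enemy flame projectile that damages the player character, MasterCharacter_BP, when its Sphere component overlaps it.
; A hit replaces this projectile's previous Wound_UI widget with a fresh one on the viewport.
; It subtracts DMG directly from CurrentHealth, bypassing the engine damage system, and snaps results below one to zero.
; The graph never destroys the projectile or removes its last wound widget.
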(event `self.Sphere.OnComponentBeginOverlap`
  (params (OverlappedComponent :type "PrimitiveComponent Object Reference") (OtherActor :type "Actor Object Reference") (OtherComp :type "PrimitiveComponent Object Reference") (OtherBodyIndex :type Integer) (bFromSweep :type Boolean) (SweepResult :type "HitResult Structure (by ref)"))
  (bind _asmaster_character_bp (cast `/Game/MAIN/Blueprints/Player/MasterCharacter_BP` OtherActor))
  (bind _woundui (`self.WoundUI`)
    (:`then`
      (`Widget.RemoveFromParent` _woundui))
    (:`else`
      _))
  (set `self.WoundUI` null)
  (bind _returnvalue (`|CreateWidget` "/Game/MAIN/UI/Wound_UI.Wound_UI_C"))
  (bind _output_get (set `self.WoundUI` _returnvalue))
  (`UserWidget.AddToViewport` _output_get 0)
  (bind _output_get_2 (set `/Game/MAIN/Blueprints/Player/MasterCharacter_BP.CurrentHealth` (- (`/Game/MAIN/Blueprints/Player/MasterCharacter_BP.CurrentHealth` _asmaster_character_bp) (`self.DMG`)) _asmaster_character_bp))
  (if (< _output_get_2 1)
    (set `/Game/MAIN/Blueprints/Player/MasterCharacter_BP.CurrentHealth` 0 _asmaster_character_bp)))

(fn `UserConstructionScript`)