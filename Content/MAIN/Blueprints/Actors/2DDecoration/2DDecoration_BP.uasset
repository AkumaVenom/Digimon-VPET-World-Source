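; 2DDecoration_BP is a non-colliding 2D sprite decoration that turns to face the player, billboard style.
; On BeginPlay it caches the player's MasterCharacter_BP and disables actor collision.
; Each tick, FacePlayer sets the PaperSprite's world rotation from a look-at toward the player, using yaw only with a 90-degree offset so the sprite stays upright.
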(event `self.ReceiveBeginPlay`
  (bind _asmaster_character_bp (cast `/Game/MAIN/Blueprints/Player/MasterCharacter_BP` (`GameplayStatics.GetPlayerCharacter` 0)))
  (set `self.PlayerReference` _asmaster_character_bp)
  (`self.SetActorEnableCollision` self false))

(event `self.ReceiveTick`
  (params (DeltaSeconds :type "Float (single-precision)"))
  (`self.FacePlayer`))

(fn `FacePlayer`
  (bind _playerreference (`self.PlayerReference`)
    (:`then`
      (bind (_returnvalue_roll _returnvalue_pitch _returnvalue_yaw) (`KismetMathLibrary.BreakRotator` (`KismetMathLibrary.FindLookAtRotation` (`SceneComponent.K2_GetComponentLocation` (`self.PaperSprite`)) (`self.K2_GetActorLocation` _playerreference))))
      (`SceneComponent.K2_SetWorldRotation` (`self.PaperSprite`) (`KismetMathLibrary.MakeRotator` 0.0 0.0 (- _returnvalue_yaw 90.0)) false false)
      (return))
    (:`else`)))

(fn `UserConstructionScript`)