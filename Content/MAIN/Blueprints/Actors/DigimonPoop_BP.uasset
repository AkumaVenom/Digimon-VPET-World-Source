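; Digimon poop actor that plays a sound when it appears and destroys itself after a one-minute delay.
; It caches the player character on BeginPlay and turns off sprite collision.
; Tick swaps between mesh and sprite to match the player's IsDigimonModels3D flag, using two cross-resetting DoOnce nodes so visibility is set only on changes.
; Tick also calls FacePlayer, a yaw-only billboard turning the sprite toward the player's follow camera.
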(event `self.ReceiveBeginPlay`
  (bind _asmaster_character_bp (cast `/Game/MAIN/Blueprints/Player/MasterCharacter_BP` (`GameplayStatics.GetPlayerCharacter` 0)))
  (set `self.PlayerReference` _asmaster_character_bp)
  (`PrimitiveComponent.SetCollisionEnabled` (`self.PoopSprite`) "NoCollision"))

(event `self.ReceiveTick`
  (params (DeltaSeconds :type "Float (single-precision)"))
  (`|ExecutionSequence`
    (:`then_0`
      (bind _playerreference (`self.PlayerReference`)
        (:`then`
          (if (`/Game/MAIN/Blueprints/Player/MasterCharacter_BP.IsDigimonModels3D` _playerreference)
            (`/Engine/EditorBlueprintResources/StandardMacros.DoOnce` false :!label _label
              (:`Completed`
                (`SceneComponent.SetVisibility` (`self.PoopMesh`) true false)
                (`SceneComponent.SetVisibility` (`self.PoopSprite`) false false)
                (goto _label_2 :!via `Reset`)))
            (else
              (`/Engine/EditorBlueprintResources/StandardMacros.DoOnce` false :!label _label_2
                (:`Completed`
                  (`SceneComponent.SetVisibility` (`self.PoopSprite`) true false)
                  (`SceneComponent.SetVisibility` (`self.PoopMesh`) false false)
                  (goto _label :!via `Reset`))))))
        (:`else`)))
    (:`then_1`
      (`/Engine/EditorBlueprintResources/StandardMacros.DoOnce` false
        (:`Completed`
          (`GameplayStatics.PlaySound2D` "/Game/MAIN/VPET/Sound/DigiPoop_Sound_Cue.DigiPoop_Sound_Cue" 1.0 1.0 0.0 null null)
          (`KismetSystemLibrary.Delay` 60.0)
          (`self.K2_DestroyActor`))))
    (:`then_2`
      (`self.PlayerReference`
        (:`then`
          (`self.FacePlayer`))
        (:`else`)))))

(fn `FacePlayer`
  (bind _poopsprite (`self.PoopSprite`))
  (bind _playerreference (`self.PlayerReference`)
    (:`then`
      (bind (_returnvalue_roll _returnvalue_pitch _returnvalue_yaw) (`KismetMathLibrary.BreakRotator` (`KismetMathLibrary.FindLookAtRotation` (`SceneComponent.K2_GetComponentLocation` _poopsprite) (`SceneComponent.K2_GetComponentLocation` (`/Game/MAIN/Blueprints/Player/MasterCharacter_BP.FollowCamera` _playerreference)))))
      (`SceneComponent.K2_SetWorldRotation` _poopsprite (`KismetMathLibrary.MakeRotator` 0.0 0.0 (- _returnvalue_yaw 90.0)) false false)
      (return))
    (:`else`)))

(fn `UserConstructionScript`)