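; SideQuestionMark_BP is a quest marker actor that keeps a question mark turned in line with the player's view, judging by its name for side quests.
; On BeginPlay it searches for MasterCharacter_BP actors and stores the last one found as the player reference.
; Tick passes through two short delays, then sets only the actor's yaw from the look-at rotation between the player's follow camera and the question mark.
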(event `self.ReceiveBeginPlay`
  (bind _outactors (`GameplayStatics.GetAllActorsOfClass` "/Game/MAIN/Blueprints/Player/MasterCharacter_BP.MasterCharacter_BP_C"))
  (for _array_element _outactors
    (set `self.PlayerReference` _array_element)))

(event `self.ReceiveTick`
  (params (DeltaSeconds :type "Float (single-precision)"))
  (bind (_returnvalue_roll _returnvalue_pitch _returnvalue_yaw) (`KismetMathLibrary.BreakRotator` (`KismetMathLibrary.FindLookAtRotation` (`SceneComponent.K2_GetComponentLocation` (`/Game/MAIN/Blueprints/Player/MasterCharacter_BP.FollowCamera` (`self.PlayerReference`))) (`SceneComponent.K2_GetComponentLocation` (`self.QuestionMark`)))))
  (`KismetSystemLibrary.Delay` 0.05)
  (`KismetSystemLibrary.Delay` 0.05)
  (`self.K2_SetActorRotation` (`KismetMathLibrary.MakeRotator` 0.0 0.0 _returnvalue_yaw)))

(fn `UserConstructionScript`)