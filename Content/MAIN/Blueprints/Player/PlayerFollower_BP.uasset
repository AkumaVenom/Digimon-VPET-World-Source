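; Companion pawn that follows the player as one of seven selectable partner characters (Tai, Matt, Sora, Mimi, Izzy, TK, Joe).
; Tick issues AIMoveTo toward the player and teleports the follower to the player's FollowerPoint when it falls too far behind.
; Shortly after BeginPlay, CalculatePartnerSkin reads the partner booleans, defaulting to Mimi.
; Each selection event sets those flags exclusively and swaps mesh, anim class and scale.
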(event `self.ReceiveBeginPlay`
  (bind _asmaster_character_bp (cast `/Game/MAIN/Blueprints/Player/MasterCharacter_BP` (`GameplayStatics.GetPlayerCharacter` 0)))
  (set `self.PlayerReference` _asmaster_character_bp)
  (`KismetSystemLibrary.Delay` 1.5)
  (`self.CalculatePartnerSkin`))

(event `self.ReceiveTick`
  (params (DeltaSeconds :type "Float (single-precision)"))
  (`|ExecutionSequence`
    (:`then_0`
      (`|AIMoveTo` self (0.0 0.0 0.0) (`self.PlayerReference`) 200.0))
    (:`then_1`
      (if (> (`self.GetDistanceTo` self (`self.PlayerReference`)) 8000.0)
        (`self.K2_SetActorLocation` self (`SceneComponent.K2_GetComponentLocation` (`/Game/MAIN/Blueprints/Player/MasterCharacter_BP.FollowerPoint` (`self.PlayerReference`))) false false)))))

(event `TaiPartnerSelected`
  (bind _mesh (`self.Mesh`))
  (set `self.IsTaiPartner` true)
  (set `self.IsMattPartner` false)
  (set `self.IsSoraPartner` false)
  (set `self.IsMimiPartner` false)
  (set `self.IsIzzyPartner` false)
  (set `self.IsTKPartner` false)
  (set `self.IsJoePartner` false)
  (`SkinnedMeshComponent.SetSkinnedAssetAndUpdate` _mesh "/Game/MAIN/VPET/3D/Player/Tai/Tai_SK.Tai_SK" true)
  (`SkeletalMeshComponent.SetAnimInstanceClass` _mesh "/Game/MAIN/VPET/3D/Player/Tai/FollowerTaiAnimBP.FollowerTaiAnimBP_C")
  (`SceneComponent.SetRelativeScale3D` _mesh (80.0 80.0 80.0)))

(event `MattPartnerSelected`
  (bind _mesh (`self.Mesh`))
  (set `self.IsTaiPartner` false)
  (set `self.IsMattPartner` true)
  (set `self.IsSoraPartner` false)
  (set `self.IsMimiPartner` false)
  (set `self.IsIzzyPartner` false)
  (set `self.IsTKPartner` false)
  (set `self.IsJoePartner` false)
  (`SkinnedMeshComponent.SetSkinnedAssetAndUpdate` _mesh "/Game/MAIN/VPET/3D/Player/Matt/Matt_SK.Matt_SK" true)
  (`SkeletalMeshComponent.SetAnimInstanceClass` _mesh "/Game/MAIN/VPET/3D/Player/Matt/FollowerMattAnimBP.FollowerMattAnimBP_C")
  (`SceneComponent.SetRelativeScale3D` _mesh (60.0 60.0 60.0)))

(event `SoraPartnerSelected`
  (bind _mesh (`self.Mesh`))
  (set `self.IsTaiPartner` false)
  (set `self.IsMattPartner` false)
  (set `self.IsSoraPartner` true)
  (set `self.IsMimiPartner` false)
  (set `self.IsIzzyPartner` false)
  (set `self.IsTKPartner` false)
  (set `self.IsJoePartner` false)
  (`SkinnedMeshComponent.SetSkinnedAssetAndUpdate` _mesh "/Game/MAIN/VPET/3D/Player/Sora/Sora_SK.Sora_SK" true)
  (`SkeletalMeshComponent.SetAnimInstanceClass` _mesh "/Game/MAIN/VPET/3D/Player/Sora/FollowerSoraAnimBP.FollowerSoraAnimBP_C")
  (`SceneComponent.SetRelativeScale3D` _mesh (105.0 105.0 105.0)))

(event `MimiPartnerSelected`
  (bind _mesh (`self.Mesh`))
  (set `self.IsTaiPartner` false)
  (set `self.IsMattPartner` false)
  (set `self.IsSoraPartner` false)
  (set `self.IsMimiPartner` true)
  (set `self.IsIzzyPartner` false)
  (set `self.IsTKPartner` false)
  (set `self.IsJoePartner` false)
  (`SkinnedMeshComponent.SetSkinnedAssetAndUpdate` _mesh "/Game/MAIN/VPET/3D/Player/Mimi/Mimi_SK.Mimi_SK" true)
  (`SkeletalMeshComponent.SetAnimInstanceClass` _mesh "/Game/MAIN/VPET/3D/Player/Mimi/FollowerMimiAnimBP.FollowerMimiAnimBP_C")
  (`SceneComponent.SetRelativeScale3D` _mesh (70.0 70.0 70.0)))

(event `IzzyPartnerSelected`
  (bind _mesh (`self.Mesh`))
  (set `self.IsTaiPartner` false)
  (set `self.IsMattPartner` false)
  (set `self.IsSoraPartner` false)
  (set `self.IsMimiPartner` false)
  (set `self.IsIzzyPartner` true)
  (set `self.IsTKPartner` false)
  (set `self.IsJoePartner` false)
  (`SkinnedMeshComponent.SetSkinnedAssetAndUpdate` _mesh "/Game/MAIN/VPET/3D/Player/Izzy/Izzy_SK.Izzy_SK" true)
  (`SkeletalMeshComponent.SetAnimInstanceClass` _mesh "/Game/MAIN/VPET/3D/Player/Izzy/FollowerIzzyAnimBP.FollowerIzzyAnimBP_C")
  (`SceneComponent.SetRelativeScale3D` _mesh (110.0 110.0 110.0)))

(event `TKPartnerSelected`
  (bind _mesh (`self.Mesh`))
  (set `self.IsTaiPartner` false)
  (set `self.IsMattPartner` false)
  (set `self.IsSoraPartner` false)
  (set `self.IsMimiPartner` false)
  (set `self.IsIzzyPartner` false)
  (set `self.IsTKPartner` true)
  (set `self.IsJoePartner` false)
  (`SkinnedMeshComponent.SetSkinnedAssetAndUpdate` _mesh "/Game/MAIN/VPET/3D/Player/TK/TK_SK.TK_SK" true)
  (`SkeletalMeshComponent.SetAnimInstanceClass` _mesh "/Game/MAIN/VPET/3D/Player/TK/FollowerTKAnimBP.FollowerTKAnimBP_C")
  (`SceneComponent.SetRelativeScale3D` _mesh (70.0 70.0 70.0)))

(event `JoePartnerSelected`
  (bind _mesh (`self.Mesh`))
  (set `self.IsTaiPartner` false)
  (set `self.IsMattPartner` false)
  (set `self.IsSoraPartner` false)
  (set `self.IsMimiPartner` false)
  (set `self.IsIzzyPartner` false)
  (set `self.IsTKPartner` false)
  (set `self.IsJoePartner` true)
  (`SkinnedMeshComponent.SetSkinnedAssetAndUpdate` _mesh "/Game/MAIN/VPET/3D/Player/Joe/Joe_SK.Joe_SK" true)
  (`SkeletalMeshComponent.SetAnimInstanceClass` _mesh "/Game/MAIN/VPET/3D/Player/Joe/FollowerJoeAnimBP.FollowerJoeAnimBP_C")
  (`SceneComponent.SetRelativeScale3D` _mesh (100.0 100.0 100.0)))

(fn `CalculatePartnerSkin`
  (if (`self.IsTaiPartner`)
    (`self.TaiPartnerSelected`)
    (return)
    (elif (`self.IsMattPartner`)
      (`self.MattPartnerSelected`)
      (return)
      (elif (`self.IsSoraPartner`)
        (`self.SoraPartnerSelected`)
        (return)
        (elif (`self.IsMimiPartner`)
          (`self.MimiPartnerSelected`)
          (return)
          (elif (`self.IsIzzyPartner`)
            (`self.IzzyPartnerSelected`)
            (return)
            (elif (`self.IsTKPartner`)
              (`self.TKPartnerSelected`)
              (return)
              (elif (`self.IsJoePartner`)
                (`self.JoePartnerSelected`)
                (return)
                (else
                  (`self.MimiPartnerSelected`)
                  (return))))))))))

(fn `UserConstructionScript`)