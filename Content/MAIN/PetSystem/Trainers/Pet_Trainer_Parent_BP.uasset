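; Parent Blueprint for pet trainer NPCs, which carry a set of pets and open a pet inventory when interacted with.
; BeginPlay copies the Pets array into the PetSystemComponent inventory by index, and Interact toggles that component's pet inventory.
; When CanFreeRoam is set, Tick uses a randomized Delay to pace AIMoveTo wandering to random reachable nearby points, tracking IsMoving until each move succeeds or fails.
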(event `self.ReceiveActorBeginOverlap`
  (params (OtherActor :type "Actor Object Reference"))
  (if true
    _))

(event `self.ReceiveTick`
  (params (DeltaSeconds :type "Float (single-precision)"))
  (if (`self.CanFreeRoam`)
    (`KismetSystemLibrary.Delay` (`KismetMathLibrary.RandomFloatInRange` 5.0 7.0))
    (set `self.IsMoving` true)
    (`|AIMoveTo` self (`NavigationSystemV1.K2_GetRandomReachablePointInRadius` (`self.K2_GetActorLocation`) 2000.0 null null) null
      (:`OnSuccess`
        _)
      (:`OnFail`
        _))
    (set `self.IsMoving` false)))

(event `/Game/MAIN/QuestSystem/InteractInterface.Interact`
  (params (Interacter :type "Actor Object Reference"))
  (`/Game/MAIN/PetSystem/PetSystemComponent.TogglePetInventory` (`self.PetSystemComponent`)))

(event `self.ReceiveBeginPlay`
  (for (_array_element _array_index) (`self.Pets`)
    (`KismetArrayLibrary.Array_Set` (`/Game/MAIN/PetSystem/PetSystemComponent.Inventory` (`self.PetSystemComponent`)) _array_index _array_element)))

(fn `UserConstructionScript`)