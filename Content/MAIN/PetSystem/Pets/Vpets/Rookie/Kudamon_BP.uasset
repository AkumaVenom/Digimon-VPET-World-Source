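; Kudamon_BP is a Rookie-tier pet in the pet system that the player can summon by using it as an item.
; Its UseItem override runs the parent logic, casts player character 0 to MasterCharacter_BP, calls SummonPet with its own class and returns true.
; The event graph holds only disabled default events, and the construction script just calls the parent.
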(fn `UseItem`
  (returns (Success :type Boolean))
  (`parent.UseItem`)
  (bind _asmaster_character_bp (cast `/Game/MAIN/Blueprints/Player/MasterCharacter_BP` (`GameplayStatics.GetPlayerCharacter` 0)))
  (`/Game/MAIN/Blueprints/Player/MasterCharacter_BP.SummonPet` _asmaster_character_bp "Kudamon_BP_C")
  (return true))

(fn `UserConstructionScript`
  (`parent.UserConstructionScript`))