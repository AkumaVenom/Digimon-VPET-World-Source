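; Player-controlled turret that fires a reflecting trace, apparently an electricity beam, from its Scene component.
; Every tick it calls Reflect on its Reflected member with a capped trace count and length, always switched on.
; On BeginPlay it enables input from the first player controller, so E and Q rotate the Cube in fixed steps in opposite directions.
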(event `self.ReceiveTick`
  (params (DeltaSeconds :type "Float (single-precision)"))
  (`/Game/ReflectedElectricity/Blueprints/Reflected.Reflect` (`self.Reflected`) 15 1555.0 (`self.Scene`) 0 true))

(event `self.ReceiveBeginPlay`
  (`self.EnableInput` (`GameplayStatics.GetPlayerController` 0)))

(event `Key|E`
  (params (Key :type "Key Structure"))
  (:`Pressed`
    (`SceneComponent.K2_AddRelativeRotation` (`self.Cube`) (struct :`Yaw` 10.0) false false)))

(event `Key|Q`
  (params (Key :type "Key Structure"))
  (:`Pressed`
    (`SceneComponent.K2_AddRelativeRotation` (`self.Cube`) (struct :`Yaw` -10.0) false false)))

(fn `UserConstructionScript`)