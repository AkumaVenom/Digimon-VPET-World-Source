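; Reflecting electricity beam that fires from a given scene component and bounces off the surfaces it hits.
; Shoot chains line traces mirrored on impact normals, up to a trace limit or a miss, spawning a beam emitter per segment.
; BeginPlay maps IDs to particle templates from DT_Particles for color selection.
; Reflect calls Shoot, clears the beams after a delay, then fires OnReflection with the last hit if anything was struck.
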(event `self.ReceiveBeginPlay`
  ;[1 1 1] Init our datatable
  (`self.Init`))

(event `Reflect`
  (params (`Max Traces` :type Integer) (TraceLenght :type "Float (double-precision)") (`Shoot From` :type "SceneComponent Object Reference") (ParticleColorID :type Integer) (`On/Off` :type Boolean))
  ;[1 1 1] Reflects and clears.
  (if `On/Off`
    (bind (_hitactor _primitivehitcomponent _hitresult _hit_success) (`self.Shoot` `Max Traces` TraceLenght `Shoot From` ParticleColorID))
    (`KismetSystemLibrary.Delay` (`self.Time Delay`))
    (`self.Clear`)
    (bind _output_get (set `self.Hit Result` _hitresult))
    (bind _output_get_2 (set `self.Hit Success` _hit_success))
    (if _output_get_2
      (`self.OnReflection` (`self.LastHitActor`) _output_get _primitivehitcomponent))))

(fn `Clear`
  (bind _particlearray (`self.ParticleArray`))
  ;[1 1 1] Here , we are getting our Beam Array which we store in our Reflect function , first we destroy it and we clear the array afterwards.
  (`self.K2_DestroyComponent` _particlearray)
  (`KismetArrayLibrary.Array_Clear` _particlearray))

(fn `Init`
  (bind _outrownames (`DataTableFunctionLibrary.GetDataTableRowNames` "/Game/ReflectedElectricity/Datatables/DT_Particles.DT_Particles"))
  (for _array_element _outrownames
    (bind _returnvalue (`|GetDataTableRow` "/Game/ReflectedElectricity/Datatables/DT_Particles.DT_Particles" _array_element)
      (:`then`
        (bind (_id _particle) (break `/Game/ReflectedElectricity/Structs/BeamInfo` _returnvalue))
        (`BlueprintMapLibrary.Map_Add` (`self.IDToParticle`) _id _particle)))))

(fn `Shoot`
  (params (MaxTraces :type Integer) (TraceLength :type "Float (double-precision)") (ShootFrom :type "SceneComponent Object Reference") (ParticleColorID :type Integer))
  (returns (HitActor :type "Actor Object Reference") (PrimitiveHitComponent :type "PrimitiveComponent Object Reference") (HitResult :type "HitResult Structure") (`Hit Success` :type Boolean))
  (locals (SecondHitStart :type "Vector Structure") (SecondHitEnd :type "Vector Structure") (LoopStart :type "Vector Structure") (HResult :type "HitResult Structure") (SelectedParticleID :type Integer))
  (bind _returnvalue (`SceneComponent.K2_GetComponentLocation` ShootFrom))
  (bind (_bblockinghit _binitialoverlap _time _distance _location _impactpoint _normal _impactnormal _physmat _hitactor _hitcomponent _hitbonename _hititem _faceindex _tracestart _traceend) (`GameplayStatics.BreakHitResult` (`local.HResult`)))
  (bind (_bblockinghit_2 _binitialoverlap_2 _time_2 _distance_2 _location_2 _impactpoint_2 _normal_2 _impactnormal_2 _physmat_2 _hitactor_2 _hitcomponent_2) (`GameplayStatics.BreakHitResult` (`local.HResult`)))
  ;[1 1 1] Here we are reflecting the first 2 hits , then we are going in into a loop where we perform linetraces and break it if it doesnt hit anything.And we store the variables that we'll need later on to pass that information on the output
  (set `local.SelectedParticleID` ParticleColorID)
  (bind (_outhit _returnvalue_2) (`KismetSystemLibrary.LineTraceSingle` _returnvalue (+ _returnvalue (* (`SceneComponent.GetForwardVector` ShootFrom) TraceLength)) (`self.TraceChannel`) (`self.TraceComplex`)))
  (if _returnvalue_2
    (set `self.Current Index` 0)
    (bind (_bblockinghit_3 _binitialoverlap_3 _time_3 _distance_3 _location_3 _impactpoint_3 _normal_3 _impactnormal_3 _physmat_3 _hitactor_3 _hitcomponent_3 _hitbonename_2 _hititem_2 _faceindex_2 _tracestart_2 _traceend_2) (`GameplayStatics.BreakHitResult` _outhit))
    (set `local.SecondHitStart` (+ _impactpoint_3 _normal_3))
    (set `local.SecondHitEnd` (+ _impactpoint_3 (`KismetMathLibrary.MirrorVectorByNormal` (- _traceend_2 _tracestart_2) _impactnormal_3)))
    (set `self.LastHitActor` _hitactor_3)
    (set `self.LastHitComponent` _hitcomponent_3)
    (set `local.HResult` _outhit)
    (bind _returnvalue_3 (`GameplayStatics.SpawnEmitterAtLocation` (`BlueprintMapLibrary.Map_Find` (`self.IDToParticle`) (`local.SelectedParticleID`))))
    (`ParticleSystemComponent.SetBeamSourcePoint` _returnvalue_3 0 (`SceneComponent.K2_GetComponentLocation` ShootFrom) 0)
    (`ParticleSystemComponent.SetBeamEndPoint` _returnvalue_3 0 (`local.SecondHitStart`))
    (`KismetArrayLibrary.Array_Add` (`self.ParticleArray`) _returnvalue_3)
    (bind (_outhit_2 _returnvalue_4) (`KismetSystemLibrary.LineTraceSingle` (`local.SecondHitStart`) (`local.SecondHitEnd`) (`self.TraceChannel`) (`self.TraceComplex`)))
    (if _returnvalue_4
      (set `self.Current Index` 1)
      (bind (_bblockinghit_4 _binitialoverlap_4 _time_4 _distance_4 _location_4 _impactpoint_4 _normal_4 _impactnormal_4 _physmat_4 _hitactor_4 _hitcomponent_4) (`GameplayStatics.BreakHitResult` _outhit_2))
      (set `self.LastHitComponent` _hitcomponent_4)
      (set `self.LastHitActor` _hitactor_4)
      (set `local.HResult` _outhit_2)
      (bind _returnvalue_5 (`GameplayStatics.SpawnEmitterAtLocation` (`BlueprintMapLibrary.Map_Find` (`self.IDToParticle`) (`local.SelectedParticleID`))))
      (`ParticleSystemComponent.SetBeamSourcePoint` _returnvalue_5 0 (`local.SecondHitStart`) 0)
      (`ParticleSystemComponent.SetBeamEndPoint` _returnvalue_5 0 _impactpoint_4)
      (`KismetArrayLibrary.Array_Add` (`self.ParticleArray`) _returnvalue_5)
      (set `local.HResult` _outhit_2)
      (for _index (range (+ (- MaxTraces 2) 1))
        (set `local.LoopStart` (+ _normal _impactpoint))
        (set `local.SecondHitEnd` (+ _impactpoint (`KismetMathLibrary.MirrorVectorByNormal` (- _traceend _tracestart) _impactnormal)))
        (bind (_outhit_3 _returnvalue_6) (`KismetSystemLibrary.LineTraceSingle` (`local.LoopStart`) (`local.SecondHitEnd`) (`self.TraceChannel`) (`self.TraceComplex`)))
        (if _returnvalue_6
          (set `self.Current Index` (+ _index 2))
          (bind (_bblockinghit_5 _binitialoverlap_5 _time_5 _distance_5 _location_5 _impactpoint_5 _normal_5 _impactnormal_5 _physmat_5 _hitactor_5 _hitcomponent_5 _hitbonename_3 _hititem_3 _faceindex_3 _tracestart_3 _traceend_3) (`GameplayStatics.BreakHitResult` _outhit_3))
          (set `local.LoopStart` (+ _impactpoint_5 _normal_5))
          (set `local.SecondHitEnd` (+ _impactpoint_5 (`KismetMathLibrary.MirrorVectorByNormal` (- _traceend_3 _tracestart_3) _impactnormal_5)))
          (set `local.HResult` _outhit_3)
          (bind _returnvalue_7 (`GameplayStatics.SpawnEmitterAtLocation` (`BlueprintMapLibrary.Map_Find` (`self.IDToParticle`) (`local.SelectedParticleID`))))
          (`ParticleSystemComponent.SetBeamSourcePoint` _returnvalue_7 0 _tracestart_3 0)
          (`ParticleSystemComponent.SetBeamEndPoint` _returnvalue_7 0 (`local.LoopStart`))
          (`KismetArrayLibrary.Array_Add` (`self.ParticleArray`) _returnvalue_7)
          (else
            (bind _returnvalue_8 (`GameplayStatics.SpawnEmitterAtLocation` (`BlueprintMapLibrary.Map_Find` (`self.IDToParticle`) (`local.SelectedParticleID`))))
            (`ParticleSystemComponent.SetBeamSourcePoint` _returnvalue_8 0 _tracestart_3 0)
            (`ParticleSystemComponent.SetBeamEndPoint` _returnvalue_8 0 _traceend_3)
            (set `self.Current Index` (+ _index 2))
            (`KismetArrayLibrary.Array_Add` (`self.ParticleArray`) _returnvalue_8)
            (break))))
      (set `self.LastHitComponent` _hitcomponent_2)
      (set `self.LastHitActor` _hitactor_2)
      (return (`self.LastHitActor`) (`self.LastHitComponent`) (`local.HResult`) true)
      (else
        (set `self.Current Index` 1)
        (bind _returnvalue_9 (`GameplayStatics.SpawnEmitterAtLocation` (`BlueprintMapLibrary.Map_Find` (`self.IDToParticle`) (`local.SelectedParticleID`))))
        (`ParticleSystemComponent.SetBeamSourcePoint` _returnvalue_9 0 (`local.SecondHitStart`) 0)
        (`ParticleSystemComponent.SetBeamEndPoint` _returnvalue_9 0 (`local.SecondHitEnd`))
        (`KismetArrayLibrary.Array_Add` (`self.ParticleArray`) _returnvalue_9)
        (return (`self.LastHitActor`) (`self.LastHitComponent`) (`local.HResult`) true)))
    (else
      (set `self.Current Index` 0)
      (bind _returnvalue_10 (`GameplayStatics.SpawnEmitterAtLocation` (`BlueprintMapLibrary.Map_Find` (`self.IDToParticle`) (`local.SelectedParticleID`))))
      (`ParticleSystemComponent.SetBeamSourcePoint` _returnvalue_10 0 (`SceneComponent.K2_GetComponentLocation` ShootFrom) 0)
      (`ParticleSystemComponent.SetBeamEndPoint` _returnvalue_10 0 _traceend_2)
      (`KismetArrayLibrary.Array_Add` (`self.ParticleArray`) _returnvalue_10)
      (return (`self.LastHitActor`) (`self.LastHitComponent`) (`local.HResult`) false))))